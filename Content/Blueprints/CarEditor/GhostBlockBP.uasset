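; GhostBlockBP is the car editor's ghost block actor, which takes on the appearance of a block chosen by ID.
; SetGhostID stores the ID, calls the parent implementation, then applies that block's mesh and material from the block library on CarEditorGameStateBP.
; The material becomes a new dynamic instance, and the color read before the swap is reapplied afterward.
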(event `self.ReceiveBeginPlay`)

(event `self.SetGhostID`
  (params (ID :type Integer))
  (bind _output_get (set `self.GhostID` ID))
  (`parent.SetGhostID` _output_get)
  (set `self.ColorTemp` (`self.GetColor`))
  (bind _ascar_editor_game_state_bp (cast `/Game/Blueprints/CarEditor/CarEditorGameStateBP` (`GameplayStatics.GetGameState`)))
  (bind _returnvalue (`BlockLibrary.GetBlock` (`CarEditorGameState.GetBlockLibrary` _ascar_editor_game_state_bp) (`self.GhostID`)))
  (`StaticMeshComponent.SetStaticMesh` (`self.StaticMeshComponent`) (`BasicBlock.StaticMesh` _returnvalue))
  (bind _returnvalue_2 (`PrimitiveComponent.CreateDynamicMaterialInstance` (`self.StaticMeshComponent`) 0 (`BasicBlock.Material` _returnvalue)))
  (`PrimitiveComponent.SetMaterial` (`self.StaticMeshComponent`) 0 _returnvalue_2)
  (`self.SetColor` (`self.ColorTemp`)))

(fn `UserConstructionScript`)