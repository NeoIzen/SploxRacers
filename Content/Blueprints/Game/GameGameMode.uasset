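; Game mode that builds the player's vehicle from saved car data when play begins.
; It loops over the game instance's PlayerCarArray, loading each entry through the player VehiclePawn's grid.
; Every result initializes that same pawn and attaches to it, after which the pawn is reset to the world origin at double scale.
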(event `self.ReceiveBeginPlay`
  (bind _asgame_instance_bp (cast `/Game/Blueprints/Game/GameInstanceBP` (`GameplayStatics.GetGameInstance`)))
  (bind _settings_playercararray (break `/Game/Blueprints/MainMenu/GameSettings` (`/Game/Blueprints/Game/GameInstanceBP.Settings` _asgame_instance_bp)))
  (for _array_element _settings_playercararray
    (bind _asvehicle_pawn (cast `VehiclePawn` (`GameplayStatics.GetPlayerPawn` 0)))
    (bind _returnvalue (`VehiclePawn.GetGrid` _asvehicle_pawn))
    (bind _returnvalue_2 (`Grid.LoadFromFile` _returnvalue _array_element))
    (`VehiclePawn.Initialize` _asvehicle_pawn _returnvalue_2)
    (`self.K2_AttachToActor` _returnvalue_2 _asvehicle_pawn "None" "KeepRelative" "KeepRelative" "KeepRelative" true)
    (`self.K2_SetActorTransform` _asvehicle_pawn (`KismetMathLibrary.MakeTransform` (0.0 0.0 0.0) (struct) (2.0 2.0 2.0)) false false)))

(fn `UserConstructionScript`)