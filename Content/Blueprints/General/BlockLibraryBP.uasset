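; Block library that registers the vehicle-building blocks available in the game: chassis pieces, wheels and a non-removable seat.
; On Initialize, one function per category calls AddBlock with a base class, ID, mesh, material and properties such as name, category and weight.
; Each category seeds a shared counter through SetNextID, then draws sequential IDs from GetNextID, giving each category its own ID range.
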(event `self.Initialize`
  (`self.InitializeChassisBlocks`)
  (`self.InitializeWheels`)
  (`self.InitializeSpecialBlocks`))

(fn `GetNextID`
  (returns (ID :type Integer))
  (bind _result (`/Engine/EditorBlueprintResources/StandardMacros.IncrementInt` (`self.CurrentID`))
    (:`  `
      (return _result))))

(fn `SetNextID`
  (params (NextID :type Integer))
  (set `self.CurrentID` (- NextID 1)))