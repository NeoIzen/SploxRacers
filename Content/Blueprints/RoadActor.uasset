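; RoadActor is a road that builds itself along its Spline in the construction script, with no active runtime logic.
; It divides the spline length by Spacing and adds a manually attached spline mesh per step, including one for the final remainder.
; Each segment gets RoadMesh, a world grid material and query-and-physics collision.
; Segment endpoints and tangents are sampled from the spline in world space, with tangents left unscaled.
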(fn `UserConstructionScript`
  (locals (Distance :type "Float (double-precision)"))
  (bind _distance (`local.Distance`))
  (bind _returnvalue (+ (`local.Distance`) (`self.Spacing`)))
  (for _index (range (+ (`.ReturnValue` (`KismetMathLibrary.FMod` (`SplineComponent.GetSplineLength` (`self.Spline`)) (`self.Spacing`))) 1))
    (set `local.Distance` (* _index (`self.Spacing`)))
    (bind _returnvalue_2 (`AddComponent|NODE_AddSplineMeshComponent-0` :`bManualAttachment` true))
    (`PrimitiveComponent.SetCollisionEnabled` _returnvalue_2 "QueryAndPhysics")
    (`StaticMeshComponent.SetStaticMesh` _returnvalue_2 "/Game/Meshes/RoadMesh.RoadMesh")
    (`PrimitiveComponent.SetMaterial` _returnvalue_2 0 "/Engine/EngineMaterials/WorldGridMaterial.WorldGridMaterial")
    (`SplineMeshComponent.SetStartAndEnd` _returnvalue_2 (`SplineComponent.GetLocationAtDistanceAlongSpline` (`self.Spline`) _distance "World") (`SplineComponent.GetTangentAtDistanceAlongSpline` (`self.Spline`) _distance "World") (`SplineComponent.GetLocationAtDistanceAlongSpline` (`self.Spline`) _returnvalue "World") (`SplineComponent.GetTangentAtDistanceAlongSpline` (`self.Spline`) _returnvalue "World") true)))